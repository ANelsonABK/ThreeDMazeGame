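; BP_SlidingDoor is a maze game door that slides open on overlap with its collision box and closes when the overlap ends.
; A timeline drives the mesh's relative Y location, playing forward to open, reversing to close, and toggling IsOpen when it finishes.
; CheckDoorStatus gates opening: a one-way door marks itself used on the first overlap and refuses to open afterward.
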(event `self.DoorCollisionBox.OnComponentBeginOverlap`
  (params (OverlappedComponent :type "PrimitiveComponent Object Reference") (OtherActor :type "Actor Object Reference") (OtherComp :type "PrimitiveComponent Object Reference") (OtherBodyIndex :type Integer) (bFromSweep :type Boolean) (SweepResult :type "HitResult Structure (by ref)"))
  (`self.CheckDoorStatus`)
  (if (`self.CanOpenDoor`)
    (bind (_direction _slidingtrack) (`Timeline|SlideDoorTimeline` :!label _label)
      (:`Update`
        (`SceneComponent.K2_SetRelativeLocation` (`self.DoorMesh`) (`KismetMathLibrary.MakeVector` 0.0 _slidingtrack) false false))
      (:`Finished`
        (set `self.IsOpen` (not (`self.IsOpen`)))))))

(event `self.DoorCollisionBox.OnComponentEndOverlap`
  (params (OverlappedComponent :type "PrimitiveComponent Object Reference") (OtherActor :type "Actor Object Reference") (OtherComp :type "PrimitiveComponent Object Reference") (OtherBodyIndex :type Integer))
  (goto _label :!via `Reverse`))

(fn `CheckDoorStatus`
  (bind _isonewaydoor (`self.IsOneWayDoor`))
  (bind _useddoor (`self.UsedDoor`))
  ;[1 1 1] Check if Door Can Open
  (if (and _isonewaydoor _useddoor)
    (set `self.CanOpenDoor` false)
    (else
      (if (and _isonewaydoor (not _useddoor))
        (set `self.UsedDoor` true))
      (set `self.CanOpenDoor` true)))
  (return))

(fn `UserConstructionScript`)