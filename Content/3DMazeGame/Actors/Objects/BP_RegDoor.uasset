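; BP_RegDoor is a maze-game door that swings open when something overlaps its Box and closes when the overlap ends.
; The OpenDoorT timeline plays or reverses on overlap, lerping DoorMesh yaw between closed and open positions and toggling IsOpen when finished.
; Interact sets the timeline play rate from open or close times, but the OpenDoor and CloseDoor events it calls are empty, so movement comes only from overlaps.
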(event `self.Box.OnComponentBeginOverlap`
  (params (OverlappedComponent :type "PrimitiveComponent Object Reference") (OtherActor :type "Actor Object Reference") (OtherComp :type "PrimitiveComponent Object Reference") (OtherBodyIndex :type Integer) (bFromSweep :type Boolean) (SweepResult :type "HitResult Structure (by ref)"))
  (bind (_direction _door_track) (`Timeline|OpenDoorT` :!label _label)
    (:`Update`
      (`SceneComponent.K2_SetRelativeRotation` (`self.DoorMesh`) (`KismetMathLibrary.MakeRotator` 0.0 0.0 (`KismetMathLibrary.Lerp` (`self.ClosePosition`) (`self.OpenPosition`) _door_track)) false false))
    (:`Finished`
      (set `self.IsOpen?` (not (`self.IsOpen?`))))))

(event `self.Box.OnComponentEndOverlap`
  (params (OverlappedComponent :type "PrimitiveComponent Object Reference") (OtherActor :type "Actor Object Reference") (OtherComp :type "PrimitiveComponent Object Reference") (OtherBodyIndex :type Integer))
  (goto _label :!via `Reverse`))

(event `CloseDoor`)

(event `OpenDoor`)

(fn `Interact`
  (params (Interactor :type "Character Object Reference"))
  (returns (DidInteract :type Boolean))
  (bind _opendoort (`self.OpenDoorT`))
  (if (not (`self.IsOpen?`))
    (`TimelineComponent.SetPlayRate` _opendoort (/ 1.0 (`self.TimeToOpen(s)`)))
    (`self.OpenDoor`)
    (else
      (`TimelineComponent.SetPlayRate` _opendoort (/ 1.0 (`self.TimeToClose(s)`)))
      (`self.CloseDoor`)))
  (return true))

(fn `UserConstructionScript`)