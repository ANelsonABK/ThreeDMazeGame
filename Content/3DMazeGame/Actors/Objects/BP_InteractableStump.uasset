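; BP_InteractableStump is a maze game stump that acts as a trigger for opening a linked button door.
; Player overlap with its TreeBox or an OnInteract event both route into Interact.
; Interact searches all BP_ButtonDoor actors for the first DoorValue matching its ButtonValue and opens it.
; It then switches the first player controller's view target to that door and sets DidInteract.
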(event `self.TreeBox.OnComponentBeginOverlap`
  (params (OverlappedComponent :type "PrimitiveComponent Object Reference") (OtherActor :type "Actor Object Reference") (OtherComp :type "PrimitiveComponent Object Reference") (OtherBodyIndex :type Integer) (bFromSweep :type Boolean) (SweepResult :type "HitResult Structure (by ref)"))
  (bind _asmgplayer_character (cast `/Game/3DMazeGame/Actors/Player/MGPlayerCharacter` OtherActor))
  (`/Game/3DMazeGame/Blueprints/InteractInterface.Interact` _asmgplayer_character))

(event `OnInteract`
  (params (Player :type "/Game/3DMazeGame/Actors/Player/MGPlayerCharacter Object Reference"))
  (`/Game/3DMazeGame/Blueprints/InteractInterface.Interact` Player))

(event `/Game/3DMazeGame/Blueprints/InteractInterface.Interact`
  (params (Interactor :type "Character Object Reference"))
  (bind _outactors (`GameplayStatics.GetAllActorsOfClass` "/Game/3DMazeGame/Actors/Objects/BP_ButtonDoor.BP_ButtonDoor_C"))
  (for _array_element _outactors
    (if (== (`/Game/3DMazeGame/Actors/Objects/BP_ButtonDoor.DoorValue` _array_element) (`self.ButtonValue`))
      (`/Game/3DMazeGame/Actors/Objects/BP_ButtonDoor.OpenDoor` _array_element Interactor)
      (`PlayerController.SetViewTargetWithBlend` (`GameplayStatics.GetPlayerController` 0) _array_element 0.0 "VTBlend_Linear" 0.0 false)
      (set `self.DidInteract` true)
      (break))))

(fn `UserConstructionScript`)